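; Player controller for the flipper game that shows or hides the pause UI.
; Its toggle-pause event fetches the HUD through BP_FlipperGameMode and sets visibility on the pause label, Restart and Resume buttons, and the overlay shared with game over.
; It only handles widget visibility; the event receives the paused state as a parameter, and BeginPlay and Tick are unused.
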(event `self.OnTogglePauseUI`
  (params (bIsPaused :type Boolean))
  (bind _asbp_flipper_game_mode (cast `/Game/Classes/BP_FlipperGameMode` (`GameplayStatics.GetGameMode`)))
  (if bIsPaused
    (bind _myhud (`/Game/Classes/BP_FlipperGameMode.MyHUD` _asbp_flipper_game_mode))
    (bind _pause (`/Game/UI/WBP_HUD.PAUSE` _myhud))
    (`Widget.SetVisibility` _pause "Visible")
    (bind _restartbutton (`/Game/UI/WBP_HUD.RestartButton` _myhud))
    (`Widget.SetVisibility` _restartbutton "Visible")
    (bind _resumebutton (`/Game/UI/WBP_HUD.ResumeButton` _myhud))
    (`Widget.SetVisibility` _resumebutton "Visible")
    (bind _gameoveroverlay (`/Game/UI/WBP_HUD.GameOverOverlay` _myhud))
    (`Widget.SetVisibility` _gameoveroverlay "Visible")
    (else
      (`Widget.SetVisibility` _pause "Hidden")
      (`Widget.SetVisibility` _restartbutton "Hidden")
      (`Widget.SetVisibility` _resumebutton "Hidden")
      (`Widget.SetVisibility` _gameoveroverlay "Hidden"))))

(fn `UserConstructionScript`)