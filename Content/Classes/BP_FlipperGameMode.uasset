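; Game mode for a flipper (pinball) game that sets up the HUD and relays game state to it.
; On BeginPlay it creates the HUD widget, shows starting lives, switches to game-only input and forces a small portrait windowed resolution.
; Lives and score update events refresh the HUD.
; Game over starts the HUD's game-over UI and hands input and the mouse cursor to the UI.
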(event `self.ReceiveBeginPlay`
  (bind _returnvalue (`|CreateWidget` "/Game/UI/WBP_HUD.WBP_HUD_C"))
  (`UserWidget.AddToViewport` _returnvalue 0)
  (bind _output_get (set `self.MyHUD` _returnvalue))
  (`/Game/UI/WBP_HUD.RefreshLives` _output_get (`self.MaxLives`))
  (`WidgetBlueprintLibrary.SetInputMode_GameOnly` (`GameplayStatics.GetPlayerController` 0))
  (bind _returnvalue_2 (`GameUserSettings.GetGameUserSettings`))
  (`GameUserSettings.SetFullscreenMode` _returnvalue_2 "Windowed")
  (`GameUserSettings.SetScreenResolution` _returnvalue_2 (make `IntPoint` 504 700))
  (`GameUserSettings.ApplySettings` _returnvalue_2 true))

(event `self.OnLivesUpdated`
  (params (NewLivesCount :type Integer))
  (`/Game/UI/WBP_HUD.RefreshLives` (`self.MyHUD`) NewLivesCount))

(event `self.OnScoreUpdated`
  (params (NewScore :type Integer))
  (`/Game/UI/WBP_HUD.RefreshScore` (`self.MyHUD`) NewScore))

(event `self.OnGameOver`
  (bind _returnvalue (`GameplayStatics.GetPlayerController` 0))
  (`/Game/UI/WBP_HUD.StartGameOverUI` (`self.MyHUD`))
  (`WidgetBlueprintLibrary.SetInputMode_UIOnlyEx` _returnvalue null)
  (set `PlayerController.bShowMouseCursor` true _returnvalue))

(fn `UserConstructionScript`)